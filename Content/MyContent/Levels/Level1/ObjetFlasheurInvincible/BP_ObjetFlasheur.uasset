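; BP_ObjetFlasheur is a flashing object with a proximity zone that flags when it can be taken.
; From BeginPlay, a looping pair of short delays endlessly swaps the Cube between its base material and the first-person projectile material.
; Box overlap events set and clear PeutPrendre without filtering the actor, printing a colored debug "Oui" or "Non".
; The graph contains no pickup action.
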(event OnComponentBeginOverlap(Box)
  (params (OverlappedComponent :type Primitive%20Component%20Object%20Reference) (OtherActor :type Actor%20Object%20Reference) (OtherComp :type Primitive%20Component%20Object%20Reference) (OtherBodyIndex :type Integer) (bFromSweep :type Boolean) (SweepResult :type Hit%20Result%20Structure%20%28by%20ref%29))
  ;[1 1 1] Check si le joueur est dans la hitbox ou non de l'objet
  (Variables|Default|SetPeutPrendre? true)
  (Development|PrintString "Oui" true true "(R=0.029119,G=1.000000,B=0.000000,A=1.000000)"))

(event OnComponentEndOverlap(Box)
  (params (OverlappedComponent :type Primitive%20Component%20Object%20Reference) (OtherActor :type Actor%20Object%20Reference) (OtherComp :type Primitive%20Component%20Object%20Reference) (OtherBodyIndex :type Integer))
  ;[1 1 1] Check si le joueur est dans la hitbox ou non de l'objet
  (Variables|Default|SetPeutPrendre? false)
  (Development|PrintString "Non" true true "(R=1.000000,G=0.006430,B=0.000000,A=1.000000)"))

(event Collision|EventActorBeginOverlap
  (params (OtherActor :type Actor%20Object%20Reference)))

(event EventBeginPlay
  ;[1 1 1] L'objet clignote dès le départ du niveau
  (Utilities|FlowControl|Delay 0.2 :!label _label)
  (Rendering|Material|SetMaterial (Variables|Default|GetCube) 0 "/Game/FPWeapon/Materials/BaseMaterial.BaseMaterial")
  (Utilities|FlowControl|Delay 0.2)
  (Rendering|Material|SetMaterial (Variables|Default|GetCube) 0 "/Game/FPWeapon/Materials/FirstPersonProjectileMaterial.FirstPersonProjectileMaterial")
  (goto _label))

(fn ConstructionScript)